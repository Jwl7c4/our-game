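; GA_EquipWeapon is a Gameplay Ability that equips a weapon on the activating character.
; On activation it spawns the Weapon actor class at the SocketName socket on the actor info's skeletal mesh and snaps it to that socket.
; It ends immediately afterward, or prints an error and ends if no valid weapon class is set.
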(event Ability|EventActivateAbility
  (bind _returnvalue (Ability|GetActorInfo))
  (if (Utilities|IsValidClass (Variables|Default|GetWeapon))
    ;[1 1 1] Spawn Weapon Actor in Socket
    (bind _returnvalue_2 (Game|SpawnActorfromClass (Variables|Default|GetWeapon) (Transformation|GetSocketTransform (.skeletalmeshcomponent _returnvalue) (Variables|Default|GetSocketName) "RTS_World") "Undefined" "MultiplyWithRoot" 0 0))
    (Transformation|AttachComponentToComponent _returnvalue_2 (.skeletalmeshcomponent _returnvalue) (Variables|Default|GetSocketName) "SnapToTarget" "SnapToTarget" "SnapToTarget" true)
    (Ability|EndAbility)
    (else
      ;[1 1 1] Weapon Class Not Set
      (Development|PrintString "ERROR - Set Mesh on equip abliity")
      (Ability|EndAbility))))

(event Ability|EventOnEndAbility
  (params (bWasCancelled :type Boolean)))