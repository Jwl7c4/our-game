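; GA_Shoot is a shooting gameplay ability whose activation and end events are empty, leaving its firing logic unconnected and never executed.
; That orphaned chain plays muzzle effect and sound, then traces from the camera to find an aim point.
; A second trace from the rifle muzzle toward that point applies the rifle's damage and spawns an impact effect, with debug line and print.
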(event Ability|EventActivateAbility
  ;[1 1 1] Shoot
)

(event Ability|EventOnEndAbility
  (params (bWasCancelled :type Boolean)))