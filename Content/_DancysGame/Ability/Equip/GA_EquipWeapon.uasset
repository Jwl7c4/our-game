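; GA_EquipWeapon is a Gameplay Ability that equips a weapon on the owning character, with weapon class and socket name supplied as variables.
; On activation it validates the class, commits without checking the result, then spawns the weapon with the controlled pawn as instigator.
; It snaps the weapon to the skeletal mesh socket and ends immediately.
; An invalid class prints an error about setting inherited variables and ends.
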(event Ability|EventActivateAbility
  (bind _returnvalue (Ability|GetActorInfo))
  ;[1 1 1] Start and Commit
  (if (Utilities|IsValidClass (Variables|Default|GetWeapon))
    (Ability|CommitAbility)
    ;[1 1 1] Spawn Weapon Actor in Socket
    (bind _returnvalue_2 (Game|SpawnActorfromClass (Variables|Default|GetWeapon) (Transformation|GetSocketTransform (.skeletalmeshcomponent _returnvalue) (Variables|Default|GetSocketName) "RTS_World") "Undefined" "MultiplyWithRoot" 0 (Pawn|GetControlledPawn (.playercontroller _returnvalue))))
    (Transformation|AttachComponentToComponent _returnvalue_2 (.skeletalmeshcomponent _returnvalue) (Variables|Default|GetSocketName) "SnapToTarget" "SnapToTarget" "SnapToTarget" true)
    (Ability|EndAbility)
    (else
      ;;[1 1 1] Weapon Class Not Set
      (Development|PrintString "ERROR - Set Inherited variables")
      (Ability|EndAbility))))

(event Ability|EventOnEndAbility
  (params (bWasCancelled :type Boolean)))